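; Enemy character that chases or shoots the player, switching by distance in a once-per-second loop started at BeginPlay.
; It moves in short AIMoveTo steps toward the player or fires aimed BP_enemy_projectile actors.
; Player projectiles and shotgun bullets kill instantly on Box overlap (head hit) or decrement Health on BodyCollision.
; Death awards score and rolls random ammo, health or weapon drops, with weapon type based on the player's WeaponNumber.
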(event OnComponentBeginOverlap(Box)
  (params (OverlappedComponent :type Primitive%20Component%20Object%20Reference) (OtherActor :type Actor%20Object%20Reference) (OtherComp :type Primitive%20Component%20Object%20Reference) (OtherBodyIndex :type Integer) (bFromSweep :type Boolean) (SweepResult :type Hit%20Result%20Structure%20%28by%20ref%29))
  (bind _asbp_first_person_projectile (Utilities|Casting|CastToBP_FirstPersonProjectile OtherActor)
    (:then
      (Utilities|FlowControl|Sequence
        (:then_0
          (Development|PrintString "Head hit"))
        (:then_1
          (Actor|DestroyActor _asbp_first_person_projectile)
          (CallFunction|Drop)
          (Actor|DestroyActor)
          (bind _asbp_first_person_character (Utilities|Casting|CastToBP_FirstPersonCharacter (Game|GetPlayerCharacter 0)))
          (Default|AddScore _asbp_first_person_character))))
    (:CastFailed
      (bind _asbp_shotgun_bullet (Utilities|Casting|CastToBP_Shotgun_Bullet OtherActor))
      (Actor|DestroyActor _asbp_shotgun_bullet)
      (CallFunction|Drop)
      (Actor|DestroyActor)
      (bind _asbp_first_person_character_2 (Utilities|Casting|CastToBP_FirstPersonCharacter (Game|GetPlayerCharacter 0)))
      (Default|AddScore _asbp_first_person_character_2))))

(event OnComponentBeginOverlap(HeadCollision)
  (params (OverlappedComponent :type Primitive%20Component%20Object%20Reference) (OtherActor :type Actor%20Object%20Reference) (OtherComp :type Primitive%20Component%20Object%20Reference) (OtherBodyIndex :type Integer) (bFromSweep :type Boolean) (SweepResult :type Hit%20Result%20Structure%20%28by%20ref%29)))

(event OnComponentBeginOverlap(BodyCollision)
  (params (OverlappedComponent :type Primitive%20Component%20Object%20Reference) (OtherActor :type Actor%20Object%20Reference) (OtherComp :type Primitive%20Component%20Object%20Reference) (OtherBodyIndex :type Integer) (bFromSweep :type Boolean) (SweepResult :type Hit%20Result%20Structure%20%28by%20ref%29))
  (bind _asbp_first_person_projectile (Utilities|Casting|CastToBP_FirstPersonProjectile OtherActor)
    (:then
      (Actor|DestroyActor _asbp_first_person_projectile)
      (CallFunction|OnBodyHit))
    (:CastFailed
      (bind _asbp_shotgun_bullet (Utilities|Casting|CastToBP_Shotgun_Bullet OtherActor))
      (Actor|DestroyActor _asbp_shotgun_bullet)
      (CallFunction|OnBodyHit))))

(event Custom|ChasePlayer
  (bind _returnvalue (Transformation|GetActorLocation))
  (AI|AIMoveTo self (+ (* (Math|Vector|Normalize (- (Transformation|GetWorldLocation (Variables|/Script/Engine.Character|GetCapsuleComponent (Game|GetPlayerCharacter 0))) _returnvalue)) (Variables|/Script/Engine.CharacterMovementComponent|GetMaxWalkSpeed (Variables|Character|GetCharacterMovement))) _returnvalue) 0 5.0 false))

(event EventBeginPlay
  (Variables|Default|SetAIControllerClass self "/Game/Blueprints/enemy_ai.enemy_ai_C")
  (Variables|/Script/Engine.CharacterMovementComponent|SetMaxWalkSpeed (Variables|Character|GetCharacterMovement) 3e+02)
  (switch Utilities|FlowControl|Switch|Switchonenemy_state (Variables|Default|GetEState) :!label _label
    (:NewEnumerator0
      (CallFunction|ShootProjectile))
    (:NewEnumerator1
      (CallFunction|ChasePlayer))
    (:NewEnumerator2
      _))
  (if (<= (Math|Vector|VectorLength (- (Transformation|GetWorldLocation (Variables|/Script/Engine.Character|GetMesh (Game|GetPlayerCharacter 0))) (Transformation|GetActorLocation))) 1e+03)
    (Variables|Default|SetEState "NewEnumerator0")
    (else
      (Variables|Default|SetEState "NewEnumerator1")))
  (Utilities|FlowControl|Delay 1.0)
  (goto _label))

(event Collision|EventActorBeginOverlap
  (params (OtherActor :type Actor%20Object%20Reference)))

(event EventTick
  (params (DeltaSeconds :type Float%20%28single-precision%29)))

(fn ConstructionScript)

(fn OnBodyHit
  (Development|PrintString "Body Hit")
  (bind _output_get (Variables|Default|SetHealth (Math|Integer|Clamp(Integer) (- (Variables|Default|GetHealth) 1) 0 4)))
  ;[1 1 1] Chance to spawn ammo or health drops
  (if (== _output_get 0)
    (Utilities|FlowControl|Sequence
      (:then_0
        (CallFunction|Drop))
      (:then_1
        (Actor|DestroyActor)
        (bind _asbp_first_person_character (Utilities|Casting|CastToBP_FirstPersonCharacter (Game|GetPlayerCharacter 0)))
        (Default|AddScore _asbp_first_person_character)))))

(fn ShootProjectile
  (bind _returnvalue (Transformation|GetActorLocation))
  (bind _returnvalue_2 (Transformation|GetActorRotation))
  (bind _returnvalue_3 (Math|Vector|GetForwardVector _returnvalue_2))
  (bind _returnvalue_4 (* _returnvalue_3 5e+01))
  (bind _returnvalue_5 (+ _returnvalue _returnvalue_4))
  (bind _returnvalue_6 (Game|SpawnActorfromClass "/Game/Blueprints/BP_enemy_projectile.BP_enemy_projectile_C" (Math|Transform|MakeTransform _returnvalue_5 "0, 0, 0" "1.000000,1.000000,1.000000") "Undefined" "MultiplyWithRoot" 0 0))
  (Game|Components|ProjectileMovement|SetVelocityinLocalSpace (Variables|/Game/Blueprints/BP_enemy_projectile.BP_enemy_projectile_C|GetProjectileMovement _returnvalue_6) (* (Math|Vector|Normalize (- (Transformation|GetActorLocation (Game|GetPlayerCharacter 0)) _returnvalue_5)) (Class|MovementComponent|GetMaxSpeed (Variables|/Game/Blueprints/BP_enemy_projectile.BP_enemy_projectile_C|GetProjectileMovement _returnvalue_6)))))

(fn Drop
  (bind _returnvalue (Transformation|GetActorLocation))
  (bind _returnvalue_2 (Math|Random|RandomIntegerinRange 0 9))
  (bind _returnvalue_3 (Math|Conversions|ToTransform(Vector) _returnvalue))
  (bind _asbp_first_person_character (Utilities|Casting|CastToBP_FirstPersonCharacter (Game|GetPlayerCharacter 0)))
  (if (or (== _returnvalue_2 0) (== _returnvalue_2 1))
    (Game|SpawnActorfromClass "/Game/Blueprints/BP_Ammo.BP_Ammo_C" _returnvalue_3 "Undefined" "MultiplyWithRoot" 0 0)
    (elif (or (== _returnvalue_2 2) (== _returnvalue_2 3))
      (Game|SpawnActorfromClass "/Game/Blueprints/BP_Health.BP_Health_C" _returnvalue_3 "Undefined" "MultiplyWithRoot" 0 0)
      (elif (== _returnvalue_2 9)
        (if (or (== (Variables|/Game/FirstPerson/Blueprints/BP_FirstPersonCharacter.BP_FirstPersonCharacter_C|GetWeaponNumber _asbp_first_person_character) 1) (== (Variables|/Game/FirstPerson/Blueprints/BP_FirstPersonCharacter.BP_FirstPersonCharacter_C|GetWeaponNumber _asbp_first_person_character) 2))
          (Game|SpawnActorfromClass "/Game/FirstPerson/Blueprints/BP_Pickup_RPG.BP_Pickup_RPG_C" _returnvalue_3 "Undefined" "MultiplyWithRoot" 0 0)
          (else
            (Game|SpawnActorfromClass "/Game/FirstPerson/Blueprints/BP_Pickup_Shotgun.BP_Pickup_Shotgun_C" _returnvalue_3 "Undefined" "MultiplyWithRoot" 0 0)))
        (elif (or (== _returnvalue_2 7) (== _returnvalue_2 8))
          (if (== (Variables|/Game/FirstPerson/Blueprints/BP_FirstPersonCharacter.BP_FirstPersonCharacter_C|GetWeaponNumber _asbp_first_person_character) 1)
            (Game|SpawnActorfromClass "/Game/FirstPerson/Blueprints/BP_Pickup_Shotgun.BP_Pickup_Shotgun_C" _returnvalue_3 "Undefined" "MultiplyWithRoot" 0 0)
            (else
              (Game|SpawnActorfromClass "/Game/FirstPerson/Blueprints/BP_Pickup_Rifle.BP_Pickup_Rifle_C" _returnvalue_3 "Undefined" "MultiplyWithRoot" 0 0))))))))